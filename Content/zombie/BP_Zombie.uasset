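; BP_Zombie is an enemy zombie that chases and melees the third-person player character.
; Pawn sensing starts an AI move to the player, and reaching them plays an attack montage guarded by IsAttacking.
; HitDetect sphere-traces at the right hand socket with debug drawing and damages the player, though nothing here calls it.
; Damage reduces Health; at zero, movement stops and a death sound plays at world origin.
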(event OnSeePawn(PawnSensing)
  (params (Pawn :type Pawn%20Object%20Reference))
  (if (and (not (Variables|Default|GetIsAttacking)) (> (Variables|Default|GetHealth) 0))
    (bind _asbp_third_person_character (Utilities|Casting|CastToBP_ThirdPersonCharacter Pawn))
    (AI|AIMoveTo self "0, 0, 0" _asbp_third_person_character 5.0 false
      (:OnSuccess
        (Variables|Default|SetIsAttacking true)
        (Animation|Montage|PlayMontage (Variables|Character|GetMesh) "/Game/zombie/AM_Zombie_attack.AM_Zombie_attack"
          (:OnCompleted
            (Variables|Default|SetIsAttacking false)))))))

(event Game|Damage|EventAnyDamage
  (params (Damage :type Float%20%28single-precision%29) (DamageType :type Damage%20Type%20Object%20Reference) (InstigatedBy :type Controller%20Object%20Reference) (DamageCauser :type Actor%20Object%20Reference))
  (Variables|Default|SetHealth (- (Variables|Default|GetHealth) Damage))
  (if (<= (Variables|Default|GetHealth) 0)
    (Pawn|Components|CharacterMovement|SetMovementMode (Variables|Character|GetCharacterMovement) "MOVE_None" 0)
    (Audio|PlaySoundatLocation "/Game/zombie/Zombie_Death.Zombie_Death" "0, 0, 0" "0, 0, 0" 1.0 1.0 0.0 0 0 0 0)))

(fn ConstructionScript)

(fn HitDetect
  (bind _mesh (Variables|Character|GetMesh))
  (bind _returnvalue (Transformation|GetSocketLocation _mesh "RightHand"))
  (bind _outhit (Collision|SphereTraceForObjects _returnvalue _returnvalue 5e+01 (Utilities|Array|MakeArray "ObjectTypeQuery9") false 0 "ForDuration"))
  (bind _asbp_third_person_character (Utilities|Casting|CastToBP_ThirdPersonCharacter (.HitActor (Collision|BreakHitResult _outhit))))
  (Game|Damage|ApplyDamage _asbp_third_person_character 1.0 0 0))